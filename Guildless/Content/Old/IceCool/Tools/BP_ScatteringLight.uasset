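; BP_ScatteringLight is a placeable actor that feeds a point light position to scattering materials through the PC_IceCool Material Parameter Collection.
; UpdateLight writes its root world location and Attenuation (as alpha) into a vector parameter named "PointLightChannel" plus its Channel value.
; It runs from the construction script and BeginPlay only, so movement during play is not tracked.
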(event `self.ReceiveBeginPlay`
  (`self.UpdateLight`))

(fn `UpdateLight`
  (bind (_returnvalue_x _returnvalue_y _returnvalue_z) (`KismetMathLibrary.BreakVector` (`SceneComponent.K2_GetComponentLocation` (`self.DefaultSceneRoot`))))
  (`KismetMaterialLibrary.SetVectorParameterValue` "/Game/Old/IceCool/Materials/Utils/PC_IceCool.PC_IceCool" (`KismetStringLibrary.Conv_StringToName` (`KismetStringLibrary.Concat_StrStr` "PointLightChannel" (`KismetStringLibrary.Conv_IntToString` (`self.Channel`)))) (make `LinearColor` _returnvalue_x _returnvalue_y _returnvalue_z (`self.Attenuation `))))

(fn `UserConstructionScript`
  (locals (NewLocalVar_0 :type Name :default "LightChannel0"))
  (`self.UpdateLight`))