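; BP_SignedDistanceField is a tool actor that renders a distance field from a source texture into a render target.
; Its Render event creates a dynamic instance of M_RenderDistanceField on the Plane component and, if a source texture is set, passes it with the search width and texture size as parameters.
; It then draws that material into RT_DistanceField, leaving the distance computation to the material.
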(event `Render`
  (bind _sourcetexture (`self.SourceTexture`))
  (bind _returnvalue (`PrimitiveComponent.CreateDynamicMaterialInstance` (`self.Plane`) 0 "/Game/Old/IceCool/Tools/Utils/M_RenderDistanceField.M_RenderDistanceField" "None"))
  (bind _output_get (set `self.MaterialInstance` _returnvalue))
  (`/Engine/EditorBlueprintResources/StandardMacros.IsValid` _sourcetexture
    (:`Is Valid`
      (`MaterialInstanceDynamic.SetTextureParameterValue` _output_get "Source" _sourcetexture)
      (`MaterialInstanceDynamic.SetScalarParameterValue` (`self.MaterialInstance`) "Width" (`KismetMathLibrary.Conv_IntToDouble` (`self.SearchWidth`)))
      (`MaterialInstanceDynamic.SetScalarParameterValue` (`self.MaterialInstance`) "TextureSize" (`KismetMathLibrary.Conv_IntToDouble` (`self.TextureSize`)))
      (`KismetRenderingLibrary.DrawMaterialToRenderTarget` "/Game/Old/IceCool/Tools/RenderTargets/RT_DistanceField.RT_DistanceField" (`self.MaterialInstance`)))))

(fn `UserConstructionScript`)