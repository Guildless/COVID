(event `self.ReceiveBeginPlay`
  (`parent.ReceiveBeginPlay`))

(event `Key|J`
  (params (Key :type "Key Structure"))
  (:`Pressed`
    (`/Engine/EditorBlueprintResources/StandardMacros.FlipFlop`
      (:`A`
        (bind _returnvalue (`|CreateWidget` "/AscentCombatFramework/ARSStatistics/UI/ARSStatisticInfo.ARSStatisticInfo_C" self (`ACFCharacter.GetStatisticsComponent` (`self.GetPossessedACFCharacter`))))
        (bind _output_get (set `self.StatInfo` _returnvalue))
        (`UserWidget.AddToViewport` _output_get 0))
      (:`B`
        (`Widget.RemoveFromParent` (`self.StatInfo`))))))

(event `Key|I`
  (params (Key :type "Key Structure"))
  (bind _returnvalue (`ACFFunctionLibrary.GetLocalACFPlayerController`))
  (:`Pressed`
    (`/Engine/EditorBlueprintResources/StandardMacros.FlipFlop`
      (:`A`
        (bind _returnvalue_2 (`|CreateWidget` "/AscentCombatFramework/Blueprints/UI/ACF_Inventory_WBP.ACF_Inventory_WBP_C" self (`ACFCharacter.GetEquipmentComponent` (`self.GetPossessedACFCharacter`))))
        (bind _output_get (set `self.Invent` _returnvalue_2))
        (`UserWidget.AddToViewport` _output_get 0)
        (`WidgetBlueprintLibrary.SetInputMode_GameAndUIEx` _returnvalue null)
        (set `self.bShowMouseCursor` true))
      (:`B`
        (`Widget.RemoveFromParent` (`self.Invent`))
        (`WidgetBlueprintLibrary.SetInputMode_GameOnly` _returnvalue)
        (set `self.bShowMouseCursor` false)))))

(fn `UserConstructionScript`
  (`parent.UserConstructionScript`))