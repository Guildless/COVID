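; Example ACF player controller that lets the player spawn companion AI groups from the keyboard.
; It references two companion group AI components, with the V and C keys each calling SpawnGroup on one of them.
; BeginPlay and the construction script only call their parent versions, and Tick is disabled.
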(event `self.ReceiveBeginPlay`
  (`parent.ReceiveBeginPlay`))

(event `Key|V`
  (params (Key :type "Key Structure"))
  (:`Pressed`
    (`ACFGroupAIComponent.SpawnGroup` (`self.ACFCompanionGroupAI`))))

(event `Key|C`
  (params (Key :type "Key Structure"))
  (:`Pressed`
    (`ACFGroupAIComponent.SpawnGroup` (`self.ACFCompanionGroupAI1`))))

(fn `UserConstructionScript`
  (`parent.UserConstructionScript`))