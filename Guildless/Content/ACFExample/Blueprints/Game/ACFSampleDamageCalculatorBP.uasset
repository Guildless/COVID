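; Sample ACF damage calculator that resolves each damage event's final damage and hit response, passing fall damage through unchanged.
; Frontal blocks trigger the attacker's impact action and drain stamina.
; Blocks, parries and dodges zero damage if the receiver can execute them.
; Otherwise hits reduce equilibrium for stagger, then apply melee or ranged damage reduced by defense, with random crit multipliers; the knockout check is never called.
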(fn `CalculateAndSetDamage`
  (returns (StructOut :type "ACFDamageEvent Structure"))
  (bind ((`contextString` _contextstring) (`DamageMultiplier` _damagemultiplier) (`DamageDealer` _damagedealer) (`DamageClass` _damageclass)) (break `ACFDamageEvent` (`self.InDamage`)))
  (if (`KismetMathLibrary.ClassIsChildOf` _damageclass "/Script/AscentCombatFramework.MeleeDamageType")
    (bind _returnvalue (`ACFFunctionLibrary.ReduceDamageByPercentage` (`ARSStatisticsComponent.GetParameterValue` (`ACFCharacter.GetStatisticsComponent` _damagedealer) (struct :`TagName` "RPG.Parameters.MeleeDamage")) (`ARSStatisticsComponent.GetParameterValue` (`Actor.GetComponentByClass` (`self.Receiver`) "/Script/AdvancedRPGSystem.ARSStatisticsComponent") (struct :`TagName` "RPG.Parameters.Defense"))))
    (set `self.damage` _returnvalue)
    (elif (`KismetMathLibrary.ClassIsChildOf` _damageclass "/Script/AscentCombatFramework.RangedDamageType")
      (bind _returnvalue_2 (`ACFFunctionLibrary.ReduceDamageByPercentage` (`ARSStatisticsComponent.GetParameterValue` (`ACFCharacter.GetStatisticsComponent` _damagedealer) (struct :`TagName` "RPG.Parameters.RangedDamage")) (`ARSStatisticsComponent.GetParameterValue` (`Actor.GetComponentByClass` (`self.Receiver`) "/Script/AdvancedRPGSystem.ARSStatisticsComponent") (struct :`TagName` "RPG.Parameters.Defense"))))
      (set `self.damage` _returnvalue_2)))
  (bind _structout (`self.SetDamage`))
  (return _structout))

(fn `CalculateFinalDamage`
  (params (inDamageEvent :type "ACFDamageEvent Structure (by ref)"))
  (returns (outFinalDamage :type "ACFDamageEvent Structure"))
  (bind ((`contextString` _contextstring) (`DamageMultiplier` _damagemultiplier) (`DamageDealer` _damagedealer) (`DamageReceiver` _damagereceiver) (`hitResult` _hitresult) (`HitResponseAction` _hitresponseaction) (`DamageClass` _damageclass) (`DamageDirection` _damagedirection)) (break `ACFDamageEvent` (`self.InDamage`)))
  (bind _output_get (set `self.InDamage` inDamageEvent))
  (`/Engine/EditorBlueprintResources/StandardMacros.IsValid` (`.DamageDealer` (break `ACFDamageEvent` _output_get))
    (:`Is Valid`
      (set `self.Receiver` _damagereceiver)
      (cast `ACFCharacter` _damagereceiver
        (:`then`
          (set `self.Direction` _damagedirection)
          (if (`KismetMathLibrary.ClassIsChildOf` _damageclass "/Script/AscentCombatFramework.FallDamageType")
            (return (`self.InDamage`))
            (else
              (`self.HandleBlock`)
              (`|SwitchGameplayTag` _hitresponseaction
                (:`Default`
                  _)
                (:`Actions.Hit`
                  _)
                (:`Actions.Parry`
                  (bind _returnvalue (`ACFActionsManagerComponent.CanExecuteAction` (`Actor.GetComponentByClass` (`self.Receiver`) "/Script/AscentCombatFramework.ACFActionsManagerComponent") (`.HitResponseAction` (break `ACFDamageEvent` (`self.InDamage`))) :!label _label))
                  (if _returnvalue
                    (bind _structout (setmembers `ACFDamageEvent` :`StructRef` (`self.InDamage`) :`FinalDamage` 0.0))
                    (return _structout)
                    (else
                      (bind _structout_2 (`self.HandleHit`))
                      (return _structout_2))))
                (:`Actions.Dodge`
                  (goto _label))
                (:`Actions.Block`
                  (goto _label))
                (:`Actions.KnockedOut`
                  (bind _structout_3 (`self.CalculateAndSetDamage`))
                  (return _structout_3))))))
        (:`CastFailed`
          _))
      (bind _structout_4 (`self.HandleHit`))
      (return _structout_4))
    (:`Is Not Valid`
      (return (`self.InDamage`)))))

(fn `HandleBlock`
  (bind (_contextstring _damagemultiplier _damagedealer) (break `ACFDamageEvent` (`self.InDamage`)))
  (bind _returnvalue (`Actor.GetComponentByClass` (`self.Receiver`) "/Script/AdvancedRPGSystem.ARSStatisticsComponent"))
  (bind _returnvalue_2 (`ARSStatisticsComponent.GetParameterValue` (`ACFCharacter.GetStatisticsComponent` _damagedealer) (struct :`TagName` "RPG.Parameters.MeleeDamage")))
  (if (and (`|EnumEquality` (`self.Direction`) "Front") (== (`ACFCharacter.GetCurrentActionState` (`ACFActionsManagerComponent.CharacterOwner` (`Actor.GetComponentByClass` (`self.Receiver`) "/Script/AscentCombatFramework.ACFActionsManagerComponent"))) (struct :`TagName` "Actions.Block")))
    (`ACFActionsManagerComponent.TriggerAction` (`ACFCharacter.GetActionsComponent` _damagedealer) (struct :`TagName` "Actions.Impact") "EHigh")
    (bind _structout (setmembers `ACFDamageEvent` :`StructRef` (`self.InDamage`) :`HitResponseAction` (struct :`TagName` "Actions.Block")))
    (set `self.InDamage` _structout)
    (`ACFFunctionLibrary.ReduceDamageByPercentage` _returnvalue_2 (`ARSStatisticsComponent.GetParameterValue` _returnvalue (struct :`TagName` "RPG.Parameters.Defense")))
    (`ARSStatisticsComponent.ModifyStatistic` _returnvalue (struct :`TagName` "RPG.Statistic.Stamina") (* _returnvalue_2 -1.0))
    (if (<= (`ARSStatisticsComponent.GetCurrentValueForStatitstic` _returnvalue (struct :`TagName` "RPG.Statistic.Stamina")) 0.0)
      (`ACFActionsManagerComponent.ExitAction` (`Actor.GetComponentByClass` (`self.Receiver`) "/Script/AscentCombatFramework.ACFActionsManagerComponent")))))

(fn `HandleHit`
  (returns (StructOut :type "ACFDamageEvent Structure (by ref)"))
  (`self.ShouldHit`)
  (bind _structout (`self.CalculateAndSetDamage`))
  (return _structout))

(fn `HandleKnockout`
  (bind (_contextstring _damagemultiplier _damagedealer _damagereceiver _physmaterial _damagezone _finaldamage _hitresult _hitdirection _hitresponseaction _damageclass) (break `ACFDamageEvent` (`self.InDamage`)))
  (bind _returnvalue (`Actor.GetComponentByClass` _damagereceiver "/Script/AdvancedRPGSystem.ARSStatisticsComponent"))
  (`/Engine/EditorBlueprintResources/StandardMacros.IsValid` _returnvalue
    (:`Is Valid`
      (if (>= (`.DamageImpulse` (defaults `Object` _damageclass)) (`ARSStatisticsComponent.GetParameterValue` _returnvalue (struct :`TagName` "RPG.Statistic.Equilibrium")))
        (setmembers `ACFDamageEvent` :`StructRef` (`self.InDamage`) :`HitResponseAction` (struct :`TagName` "Actions.KnockedOut"))))))

(fn `SetDamage`
  (returns (StructOut :type "ACFDamageEvent Structure (by ref)"))
  (locals (Mult :type "Float (double-precision)" :default 0.0) (Context :type Name :default "None"))
  (bind (_indamage_contextstring _indamage_damagemultiplier _indamage_damagedealer _indamage_damagereceiver _indamage_physmaterial _indamage_damagezone) (break `ACFDamageEvent` (`self.InDamage`)))
  (set `local.Mult` _indamage_damagemultiplier)
  (set `local.Context` _indamage_contextstring)
  (if (`|EnumEquality` _indamage_damagezone "EHighDamage")
    (set `local.Context` "Critical! "))
  (if (< (`KismetMathLibrary.RandomFloatInRange` 0.0 100.0) (`ARSStatisticsComponent.GetParameterValue` (`ACFCharacter.GetStatisticsComponent` _indamage_damagedealer) (struct :`TagName` "RPG.Parameters.CritChance")))
    (set `local.Mult` 1.5)
    (set `local.Context` " Crit!  "))
  (bind _structout (setmembers `ACFDamageEvent` :`StructRef` (`self.InDamage`) :`contextString` (`local.Context`) :`DamageMultiplier` (`local.Mult`) :`FinalDamage` (`self.damage`)))
  (return _structout))

(fn `ShouldHit`
  (bind _returnvalue (`Actor.GetComponentByClass` (`self.Receiver`) "/Script/AdvancedRPGSystem.ARSStatisticsComponent"))
  (`ARSStatisticsComponent.ModifyStatistic` _returnvalue (struct :`TagName` "RPG.Statistic.Equilibrium") (* (`ARSStatisticsComponent.GetParameterValue` _returnvalue (struct :`TagName` "RPG.Parameters.StaggerChance")) -1.0))
  (if (> (`ARSStatisticsComponent.GetCurrentValueForStatitstic` _returnvalue (struct :`TagName` "RPG.Statistic.Equilibrium")) 0.0)
    (setmembers `ACFDamageEvent` :`StructRef` (`self.InDamage`) :`HitResponseAction` (struct))
    (else
      (setmembers `ACFDamageEvent` :`StructRef` (`self.InDamage`) :`HitResponseAction` (struct :`TagName` "Actions.Hit")))))