(event `self.ReceiveBeginPlay`
  (`parent.ReceiveBeginPlay`))

(event `Key|J`
  (params (Key :type "Key Structure"))
  (:`Pressed`
    (`/Engine/EditorBlueprintResources/StandardMacros.FlipFlop`
      (:`A`
        (bind _returnvalue (`|CreateWidget` "/AscentCombatFramework/ARSStatistics/UI/ARSStatisticInfo.ARSStatisticInfo_C" self (`ACFCharacter.GetStatisticsComponent` (`self.GetPossessedACFCharacter`))))
        (bind _output_get (set `self.StatInfo` _returnvalue))
        (`UserWidget.AddToViewport` _output_get 0))
      (:`B`
        (`Widget.RemoveFromParent` (`self.StatInfo`))))))

(event `Key|I`
  (params (Key :type "Key Structure"))
  (bind _returnvalue (`self.K2_GetPawn`))
  (bind _wbp_inventory (`self.WBP_Inventory`))
  (bind _wbp_inventory_2 (`self.WBP_Inventory`))
  ;[0.04747 0.01109 0.2031] EPICO INVENTORY CODE @_@
  (:`Pressed`
    (`/Engine/EditorBlueprintResources/StandardMacros.FlipFlop`
      (:`A`
        (`/Engine/EditorBlueprintResources/StandardMacros.IsValid` _returnvalue
          (:`Is Valid`
            (`/Engine/EditorBlueprintResources/StandardMacros.IsValid` (`self.WBP_Inventory`)
              (:`Is Valid`
                _)
              (:`Is Not Valid`
                (bind _returnvalue_2 (`|CreateWidget` "/Game/ACFExample/UI/Widgets/WBP_Inventory.WBP_Inventory_C" self _returnvalue))
                (set `self.WBP_Inventory` _returnvalue_2)))
            (`UserWidget.AddToViewport` _wbp_inventory 0)
            (set `self.bShowMouseCursor` true)
            (`WidgetBlueprintLibrary.SetInputMode_GameAndUIEx` self _wbp_inventory))))
      (:`B`
        (`/Engine/EditorBlueprintResources/StandardMacros.IsValid` _wbp_inventory_2
          (:`Is Valid`
            (`Widget.RemoveFromParent` _wbp_inventory_2)
            (set `self.bShowMouseCursor` false)
            (`WidgetBlueprintLibrary.SetInputMode_GameOnly` self)))))))

(fn `UserConstructionScript`
  (`parent.UserConstructionScript`))