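; Example Ascent Combat Framework game mode that splits joining players across multiple combat teams.
; On PostLogin, it casts the new controller to ACFPlayerController and sets its CombatTeam from the NextTeam variable.
; NextTeam then advances through the ETeam enum and wraps back to ETeam1 past the upper limit, giving round-robin assignment.
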(event `self.K2_PostLogin`
  (params (NewPlayer :type "PlayerController Object Reference"))
  (bind _nextteam (`self.NextTeam`))
  (bind _returnvalue (+ _nextteam 1))
  (bind _asacfplayer_controller (cast `ACFPlayerController` NewPlayer))
  (set `ACFPlayerController.CombatTeam` _nextteam _asacfplayer_controller)
  (if (> _returnvalue 3)
    (set `self.NextTeam` "ETeam1")
    (else
      (set `self.NextTeam` (cast `ETeam` _returnvalue)))))

(fn `UserConstructionScript`
  (`parent.UserConstructionScript`))