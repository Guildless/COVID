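; Player mage character Blueprint for the ACF mage example, mapping spell inputs to named abilities.
; On BeginPlay it initializes its ACF shooting component with itself as owner and its mesh.
; Shoot, Heal and Summon input actions ask the ACF ability system to try the Curse, Bless and Summon abilities.
; The Blueprint only triggers abilities by name and has no construction or tick logic.
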(event `self.ReceiveBeginPlay`
  (`ACFShootingComponent.SetupShootingComponent` (`self.ACFShooting`) self (`self.Mesh`)))

(event `InputAction|Shoot`
  (params (Key :type "Key Structure"))
  (:`Pressed`
    (`ACFAbilitySystemComponent.TryUseAbility` (`self.ACFAbilitySystem`) "Curse")))

(event `InputAction|Heal`
  (params (Key :type "Key Structure"))
  (:`Pressed`
    (`ACFAbilitySystemComponent.TryUseAbility` (`self.ACFAbilitySystem`) "Bless")))

(event `InputAction|Summon`
  (params (Key :type "Key Structure"))
  (:`Pressed`
    (`ACFAbilitySystemComponent.TryUseAbility` (`self.ACFAbilitySystem`) "Summon")))

(fn `UserConstructionScript`)