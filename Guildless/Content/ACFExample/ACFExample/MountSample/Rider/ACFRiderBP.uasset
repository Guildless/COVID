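; ACFRiderBP is the player character Blueprint in the ACF mount sample, adding horse riding controls through an ACFRider component.
; While riding, turn, sprint and brake axes are forwarded to the ACFMountBP mount, and dodging is disabled.
; Riding state changes start or stop the "OnHorse" camera event.
; The call-horse input plays a whistle and sends a ComeHere command through the player controller's companions component.
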(event `InputAxis|MoveRight`
  (params (AxisValue :type "Float (single-precision)"))
  (bind _acfrider (`self.ACFRider`))
  (if (`ACFRiderComponent.IsRiding` _acfrider)
    (bind _asacfmount_bp (cast `/Game/ACFExample/MountSample/Mounts/ACFMountBP` (`ACFRiderComponent.GetMount` _acfrider)))
    (`/Game/ACFExample/MountSample/Mounts/ACFMountBP.Turn` _asacfmount_bp AxisValue)
    (else
      (`ACFLocomotionComponent.MoveRight` (`self.LocomotionComp`) AxisValue))))

(event `InputAction|Dodge`
  (params (Key :type "Key Structure"))
  (:`Pressed`
    (if (not (`ACFRiderComponent.IsRiding` (`self.ACFRider`)))
      (`self.TriggerAction` (struct :`TagName` "Actions.Dodge") "ELow"))))

(event `InputAxis|Sprint`
  (params (AxisValue :type "Float (single-precision)"))
  (if (`ACFRiderComponent.IsRiding` (`self.ACFRider`))
    (`self.SendAccelerateToHorse` AxisValue)))

(event `SendAccelerateToHorse`
  (params (AccelValue :type "Float (double-precision)"))
  (bind _asacfmount_bp (cast `/Game/ACFExample/MountSample/Mounts/ACFMountBP` (`ACFRiderComponent.GetMount` (`self.ACFRider`))))
  (`/Game/ACFExample/MountSample/Mounts/ACFMountBP.Accelerate` _asacfmount_bp AccelValue))

(event `self.ACFRider.OnRidingStateChanged`
  (params (bIsRiding :type Boolean))
  (if bIsRiding
    (`CCMCameraFunctionLibrary.TriggerCameraEvent` "OnHorse")
    (else
      (`CCMCameraFunctionLibrary.StopCameraEvent` "OnHorse"))))

(event `InputAxis|Brake`
  (params (AxisValue :type "Float (single-precision)"))
  (bind _acfrider (`self.ACFRider`))
  (if (`ACFRiderComponent.IsRiding` _acfrider)
    (bind _asacfmount_bp (cast `/Game/ACFExample/MountSample/Mounts/ACFMountBP` (`ACFRiderComponent.GetMount` _acfrider)))
    (`/Game/ACFExample/MountSample/Mounts/ACFMountBP.Brake` _asacfmount_bp AxisValue)))

(event `InputAction|Callhorse`
  (params (Key :type "Key Structure"))
  (:`Pressed`
    (`GameplayStatics.PlaySoundAtLocation` "/Game/ACFExample/MountSample/whistle_Cue.whistle_Cue" (`self.K2_GetActorLocation`) (struct) 1.0 1.0 0.0 null null null)
    (`ACFGroupAIComponent.SendCommandToCompanions` (`ACFPlayerController.GetCompanionsComponent` (`ACFFunctionLibrary.GetLocalACFPlayerController`)) (struct :`TagName` "AICommand.ComeHere"))))

(fn `UserConstructionScript`
  (`parent.UserConstructionScript`))