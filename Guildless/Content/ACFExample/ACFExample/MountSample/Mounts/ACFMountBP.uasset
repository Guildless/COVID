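; An ACF mount character, with horse camera events, that pawns can interact with to ride.
; Interaction starts or stops mounting through ACFMountComp, and the rider's Interact input triggers a high-priority Dismount action on the rider.
; Accelerate, Brake and Turn drive the locomotion component, with turn rate scaled by the last acceleration input.
; Leaving the mounted state stops the jog and sprint camera events.
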(event `self.ReceiveBeginPlay`
  (`parent.ReceiveBeginPlay`))

(event `self.ReceiveTick`
  (params (DeltaSeconds :type "Float (single-precision)"))
  (`parent.ReceiveTick` DeltaSeconds))

(event `InputAction|Interact`
  (params (Key :type "Key Structure"))
  (:`Pressed`
    (bind _asacfcharacter (cast `ACFCharacter` (`ACFMountComponent.GetRider` (`self.ACFMountComp`))))
    (`self.TriggerAction` _asacfcharacter (struct :`TagName` "Actions.Dismount") "EHigh")))

(event `ACFInteractableInterface.OnInteractedByPawn`
  (params (Pawn :type "Pawn Object Reference"))
  (bind _acfmountcomp (`self.ACFMountComp`))
  (bind _asacfcharacter (cast `ACFCharacter` Pawn))
  (if (`ACFMountComponent.IsMounted` _acfmountcomp)
    (`ACFMountComponent.StopMount` _acfmountcomp (`self.defDismouunt`))
    (else
      (`ACFMountComponent.StartMount` _acfmountcomp _asacfcharacter))))

(event `self.ACFMountComp.OnMountedStateChanged`
  (params (inIsMounted :type Boolean))
  (if (not inIsMounted)
    (`CCMCameraFunctionLibrary.StopCameraEvent` "HorseJog")
    (`CCMCameraFunctionLibrary.StopCameraEvent` "HorseSprint")))

(fn `Accelerate`
  (params (Value :type "Float (double-precision)"))
  (`ACFLocomotionComponent.MoveForwardLocal` (`self.LocomotionComp`) Value)
  (set `self.ScalingFactorRotation` (* Value 0.6)))

(fn `Brake`
  (params (Value :type "Float (double-precision)"))
  (`ACFLocomotionComponent.MoveForwardLocal` (`self.LocomotionComp`) (* -1 Value)))

(fn `CanBeInteracted`
  (params (Pawn :type "Pawn Object Reference"))
  (returns (ReturnValue :type Boolean))
  (return true))

(fn `GetInteractableName`
  (returns (ReturnValue :type Text))
  (return (`self.GetCharacterName`)))

(fn `Turn`
  (params (A :type "Float (double-precision)"))
  (`ACFLocomotionComponent.TurnAtRateLocal` (`self.LocomotionComp`) (* (+ 1.0 (`self.ScalingFactorRotation`)) A)))

(fn `UserConstructionScript`
  (`parent.UserConstructionScript`))