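; Rideable mount Blueprint from the ACF mount sample that a pawn can board by interacting with it.
; Interaction starts the ACFMount component with the interacting ACF character, or dismounts if already mounted, as does Interact input, also stopping the Sprint camera event.
; Attack input triggers the mount's attack action.
; Interaction is allowed only for the group lead of the mount's AI controller, and the interactable name is blank.
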(event `InputAction|Interact`
  (params (Key :type "Key Structure"))
  (:`Pressed`
    (`ACFMountComponent.StopMount` (`self.ACFMount`) (`self.defDismouunt`) :!label _label)
    (`CCMCameraFunctionLibrary.StopCameraEvent` "Sprint")))

(event `ACFInteractableInterface.OnInteractedByPawn`
  (params (Pawn :type "Pawn Object Reference"))
  (bind _asacfcharacter (cast `ACFCharacter` Pawn))
  (if (`ACFMountComponent.IsMounted` (`self.ACFMount`))
    (goto _label)
    (else
      (`ACFMountComponent.StartMount` (`self.ACFMount`) _asacfcharacter))))

(event `self.ReceivePossessed`
  (params (NewController :type "Controller Object Reference"))
  (`parent.ReceivePossessed` NewController))

(event `InputAction|Attack`
  (params (Key :type "Key Structure"))
  (:`Pressed`
    (`self.TriggerAction` (struct :`TagName` "Actions.Attack") "EMedium")))

(event `InputAction|Jump`
  (params (Key :type "Key Structure")))

(fn `CanBeInteracted`
  (params (Pawn :type "Pawn Object Reference"))
  (returns (ReturnValue :type Boolean))
  (bind _asacfaicontroller (cast `ACFAIController` (`self.GetController`)))
  (return (== (`ACFGroupAIComponent.groupLead` (`ACFAIController.GetGroup` _asacfaicontroller)) Pawn)))

(fn `GetInteractableName`
  (returns (ReturnValue :type Text))
  (return ""))

(fn `UserConstructionScript`
  (`parent.UserConstructionScript`))