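; ACFExecutionerPlayerBP is an example player Blueprint from the ACF example content that adds executions to the attack input.
; Pressing Attack first asks the ACFExecutor component to execute its current target.
; If that attempt fails, it falls back to triggering the standard Actions.Attack action.
; The other event nodes are disabled stubs, and the construction script only calls its parent.
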(event `InputAction|Attack`
  (params (Key :type "Key Structure"))
  (:`Pressed`
    (bind _returnvalue (`ACFExecutorComponent.TryExecuteCurrentTarget` (`self.ACFExecutor`)))
    (if (not _returnvalue)
      (`self.TriggerAction` (struct :`TagName` "Actions.Attack") "ENone"))))

(fn `UserConstructionScript`
  (`parent.UserConstructionScript`))