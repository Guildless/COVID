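; Reload action for ACF characters that refills the magazine of an equipped semi-automatic gun from the Ammo equipment slot.
; On start, it switches the owner to the rifle moveset and casts the current main weapon to the gun class.
; If any ammo is equipped, it requests consumption of the missing rounds and sets the magazine to full, even when fewer remain.
; Missing equipment, slot or ammo only prints a debug message.
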(event `self.OnActionStarted`
  (bind _characterowner (`self.CharacterOwner`))
  (bind _equipmentcomp (`ACFCharacter.EquipmentComp` _characterowner))
  (bind (_outslot _returnvalue) (`ACFEquipmentComponent.GetEquippedItemSlot` _equipmentcomp (struct :`TagName` "ItemSlot.Ammo")))
  (bind ((`Item` _item) (`Count` _count)) (break `InventoryItem` _outslot))
  ;[0.04747 0.01109 0.2031] Geting the main weapon and casting to the semi automatic gun.
  (`parent.OnActionStarted`)
  (`/Engine/EditorBlueprintResources/StandardMacros.IsValid` _equipmentcomp
    (:`Is Valid`
      (`ACFCharacter.SwitchMovementType` _characterowner (struct :`TagName` "Moveset.Rifle"))
      (bind _assemi__automatic_gun (cast `/Game/ACFExample/SharedAssets/Blueprints/Weapons/Semi-AutomaticGun` (`ACFEquipmentComponent.GetCurrentMainWeapon` _equipmentcomp)))
      ;[0.04747 0.01109 0.2031] Getting the ammo equipped in the slot and getting it's count to check if it's higher than 0. If it is then we consume the ammount of ammo missing from the magazine.
      (if _returnvalue
        (if (> _count 0)
          (bind _ammoinmag (`/Game/ACFExample/SharedAssets/Blueprints/Weapons/Semi-AutomaticGun.AmmoInMag` _assemi__automatic_gun))
          (bind _returnvalue_2 (- (`/Game/ACFExample/SharedAssets/Blueprints/Weapons/Semi-AutomaticGun.SizeOfMag` _assemi__automatic_gun) _ammoinmag))
          (`ACFEquipmentComponent.ConsumeItems` _equipmentcomp (`|MakeArray` (make `BaseItem` (`GameplayStatics.GetObjectClass` _item) (`KismetMathLibrary.Conv_IntToByte` _returnvalue_2))))
          ;[0.04747 0.01109 0.2031] Set the ammo in magazine to be AmmoInMag + the ammount that was missing.
          (set `/Game/ACFExample/SharedAssets/Blueprints/Weapons/Semi-AutomaticGun.AmmoInMag` (+ _ammoinmag _returnvalue_2) _assemi__automatic_gun)
          (else
            (`KismetSystemLibrary.PrintString` "There's No ammo.")))
        (else
          (`KismetSystemLibrary.PrintString` "Ammo is not equipped"))))
    (:`Is Not Valid`
      (`KismetSystemLibrary.PrintString` "CharacterOwner's Equipment Component was invalid."))))