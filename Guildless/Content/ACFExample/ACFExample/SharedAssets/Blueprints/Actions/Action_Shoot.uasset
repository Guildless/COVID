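; Ascent Combat Framework example action that fires the character's semi-automatic gun when the action starts.
; It gets the current main weapon from the owner's equipment component and casts it to the semi-automatic gun, doing nothing more if the cast fails.
; With ammo in the magazine it shoots and decrements the clamped count; otherwise it prints an empty-magazine message.
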(event `self.OnActionStarted`
  ;[0.04747 0.01109 0.2031] Getting the main weapon and casting to the semi-automatic gun.
  (`parent.OnActionStarted`)
  (bind _assemi__automatic_gun (cast `/Game/ACFExample/SharedAssets/Blueprints/Weapons/Semi-AutomaticGun` (`ACFEquipmentComponent.GetCurrentMainWeapon` (`ACFCharacter.EquipmentComp` (`self.CharacterOwner`)))))
  (bind _ammoinmag (`/Game/ACFExample/SharedAssets/Blueprints/Weapons/Semi-AutomaticGun.AmmoInMag` _assemi__automatic_gun))
  ;[0.04747 0.01109 0.2031] Shooting if the AmmoInMag is > 0 and setting the AmmoInMag to clamped value.
  (if (> _ammoinmag 0)
    (`ACFRangedWeapon.Shoot` _assemi__automatic_gun 1.0)
    (set `/Game/ACFExample/SharedAssets/Blueprints/Weapons/Semi-AutomaticGun.AmmoInMag` (`KismetMathLibrary.Clamp` (- _ammoinmag 1) 0 (`/Game/ACFExample/SharedAssets/Blueprints/Weapons/Semi-AutomaticGun.SizeOfMag` _assemi__automatic_gun)) _assemi__automatic_gun)
    (else
      (`KismetSystemLibrary.PrintString` "There's no Ammo in the magazine!" true true (struct :`G` 0.66 :`B` 1.0 :`A` 1.0) 5.0))))