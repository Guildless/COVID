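; MPrefab is a prefab actor that records the materials of its mesh components so they can be restored.
; Its construction script optionally locks actor scale to one, then caches each descendant mesh component's materials and class name in MeshCompMaterials.
; ResetMaterialsPrefab reapplies those cached materials, while ResetMaterialsOriginal restores static mesh components to their mesh asset defaults.
; The event graph is empty, and the stored LOD count is always zero.
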(fn `F_LockPrefabScale`
  (if (`self.LockPrefabScale`)
    (`self.SetActorScale3D` (1.0 1.0 1.0))))

(fn `F_StoreMeshCompData`
  (`BlueprintMapLibrary.Map_Clear` (`self.MeshCompMaterials`))
  (for _array_element (`SceneComponent.GetChildrenComponents` (`self.DefaultSceneRoot`) true)
    (bind _asmesh_component (cast `MeshComponent` _array_element))
    (`BlueprintMapLibrary.Map_Add` (`self.MeshCompMaterials`) _asmesh_component (make `/Game/GuildLessProto/Blueprints/Prefabs/Ressources/ST_MeshComponentData` (`MeshComponent.GetMaterials` _asmesh_component) 0 (`KismetStringLibrary.Conv_StringToName` (`KismetSystemLibrary.GetClassDisplayName` (`GameplayStatics.GetObjectClass` _asmesh_component)))))))

(fn `ResetMaterialsOriginal`
  (bind _keys (`BlueprintMapLibrary.Map_Keys` (`self.MeshCompMaterials`)))
  (for _array_element _keys
    (bind _asstatic_mesh_component (cast `StaticMeshComponent` _array_element))
    (for _index (range (`PrimitiveComponent.GetNumMaterials` _asstatic_mesh_component))
      (`PrimitiveComponent.SetMaterial` _asstatic_mesh_component _index (`StaticMesh.GetMaterial` (`StaticMeshComponent.StaticMesh` _asstatic_mesh_component) _index)))))

(fn `ResetMaterialsPrefab`
  (bind _meshcompmaterials (`self.MeshCompMaterials`))
  (bind _keys (`BlueprintMapLibrary.Map_Keys` _meshcompmaterials))
  (for _array_element _keys
    (bind (_value _returnvalue) (`BlueprintMapLibrary.Map_Find` _meshcompmaterials _array_element))
    (if _returnvalue
      (for (_array_element_2 _array_index) (`.Materials_4_F30F0C914B5F2EDC97FECBBA25B7BAE9` (break `/Game/GuildLessProto/Blueprints/Prefabs/Ressources/ST_MeshComponentData` _value))
        (`PrimitiveComponent.SetMaterial` _array_element _array_index _array_element_2)))))

(fn `UserConstructionScript`
  (`self.F_LockPrefabScale`)
  (`self.F_StoreMeshCompData`))