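; GrappleAction_BP is the grapple action Blueprint for a character, extending a parent action class that supplies the underlying logic.
; It calls the parent on action start and on sub-action state changes, setting the owning character's IsReeling flag on state entry and clearing it on exit.
; Leftover unconnected nodes for velocity-facing rotation, a timed camera event and a debug print never run.
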(event `self.OnActionStarted`
  (`parent.OnActionStarted`))

(event `self.OnSubActionStateEntered`
  (`parent.OnSubActionStateEntered`)
  (set `ACFCharacter.bIsReeling` true (`self.CharacterOwner`)))

(event `self.OnSubActionStateExited`
  (`parent.OnSubActionStateExited`)
  (set `ACFCharacter.bIsReeling` false (`self.CharacterOwner`)))