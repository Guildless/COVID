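; Grapple hook projectile that flies until it hits something, then stops and sticks to the component it struck.
; After a delay from spawn, a timeline ramps up the projectile's gravity scale.
; Until impact, Tick grows the collision sphere's radius with flight time up to a clamped maximum; the hit then disables that collision.
; A DestroyHook event removes the actor.
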(event `self.ReceiveHit`
  (params (MyComp :type "PrimitiveComponent Object Reference") (Other :type "Actor Object Reference") (OtherComp :type "PrimitiveComponent Object Reference") (bSelfMoved :type Boolean) (HitLocation :type "Vector Structure") (HitNormal :type "Vector Structure") (NormalImpulse :type "Vector Structure") (Hit :type "HitResult Structure (by ref)"))
  (bind _projectilemovement (`self.ProjectileMovement`))
  ;[1 1 1] Stop Movement immediately when the projectile hit something, and attach the root to the actor that has been hit
  (set `self.Hit Something?` true)
  (`MovementComponent.StopMovementImmediately` _projectilemovement)
  (`ActorComponent.Deactivate` _projectilemovement)
  (`PrimitiveComponent.SetCollisionEnabled` (`self.Sphere`) "NoCollision")
  (`self.K2_AttachToComponent` (`.HitComponent` (`GameplayStatics.BreakHitResult` Hit)) "None" "KeepWorld" "KeepRelative" "KeepRelative"))

(event `self.ReceiveBeginPlay`
  (set `self.Initial Time` (`GameplayStatics.GetTimeSeconds`))
  ;[1 1 1] Rise the gravity after a certain time
  (set `self.Initial Position` (`self.K2_GetActorLocation`))
  (`KismetSystemLibrary.Delay` (`self.Delay Before Gravity Rise`))
  (bind (_direction _gravity_scale) (`Timeline|Gravity Scale`)
    (:`Update`
      (set `ProjectileMovementComponent.ProjectileGravityScale` _gravity_scale (`self.ProjectileMovement`)))))

(event `Destroy Hook`
  ;[1 1 1] Destroy the Hook
  (`self.K2_DestroyActor`))

(event `self.ReceiveTick`
  (params (DeltaSeconds :type "Float (single-precision)"))
  (if (not (`self.Hit Something?`))
    (`SphereComponent.SetSphereRadius` (`self.Sphere`) (`KismetMathLibrary.MapRangeClamped` (- (`GameplayStatics.GetTimeSeconds`) (`self.Initial Time`)) 0.0 2.0 1.0 1000.0) true)))

(fn `UserConstructionScript`)