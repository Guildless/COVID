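; BP_GrappleHook is a grapple hook projectile that launches itself toward a target actor when it spawns.
; On BeginPlay it records its own location and the Target's location, then derives a normalized direction between them.
; It sets the ProjectileMovement velocity to that direction scaled by Speed, aiming once with no further updates in its graph.
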(event `self.ReceiveBeginPlay`
  (set `self.StartingLocation` (`self.K2_GetActorLocation`))
  (set `self.EndingLocation` (`self.K2_GetActorLocation` (`self.Target`)))
  (set `self.Direction` (`KismetMathLibrary.Normal` (- (`self.EndingLocation`) (`self.StartingLocation`))))
  (set `MovementComponent.Velocity` (* (`self.Direction`) (`self.Speed`)) (`self.ProjectileMovement`)))

(fn `UserConstructionScript`)