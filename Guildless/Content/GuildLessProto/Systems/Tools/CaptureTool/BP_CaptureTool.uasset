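; BP_CaptureTool is a scene capture tool that renders its view to a render target and exports it as an image file or texture asset.
; Capture creates a configured render target, applies projection and render settings to the SceneCaptureComponent2D, then captures.
; Export optionally writes the raw file and creates an editor-only static texture, warning instead when that uasset already exists at the current level's path.
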(fn `Capture`
  (bind _scenecapturecomponent2d (`self.SceneCaptureComponent2D`))
  (bind _returnvalue (`/Game/GuildLessProto/Systems/TechArt_FunctionLibrary.TA_CreateRenderTarget` (`self.RenderTargetSizeX`) (`self.RenderTargetSizeY`) (`self.RenderTargetFormat`) (`self.RenderTargetCompression`) (`self.RenderTargetAdress`) (`self.RenderTarget_sRGB`)))
  (bind _output_get (set `self.RenderTarget` _returnvalue))
  (set `SceneCaptureComponent2D.TextureTarget` _output_get _scenecapturecomponent2d)
  (`/Game/GuildLessProto/Systems/TechArt_FunctionLibrary.TA_SetupCaptureSceneComp` _scenecapturecomponent2d (`self.CaptureSource`) (`self.CompositeMode`) (`self.RenderMode`) (`self.ProjectionType`) (`self.ProjectionWidth`))
  (`SceneCaptureComponent2D.CaptureScene` _scenecapturecomponent2d))

(fn `Export`
  (bind _rendertarget (`self.RenderTarget`))
  (bind _rawexportname (`self.RawExportName`))
  (bind _rawexportname_2 (`self.RawExportName`))
  (bind _returnvalue (`KismetStringLibrary.Concat_StrStr` (`/Game/GuildLessProto/Systems/TechArt_FunctionLibrary.TA_GetCurrentLevelPath`) _rawexportname_2 ".uasset"))
  (`/Engine/EditorBlueprintResources/StandardMacros.IsValid` _rendertarget
    (:`Is Valid`
      (`|ExecutionSequence`
        (:`then_0`
          (if (`self.ExportRaw`)
            (`KismetRenderingLibrary.ExportRenderTarget` _rendertarget (`self.RawExportPath`) (`KismetStringLibrary.Concat_StrStr` _rawexportname (select `bool` (`KismetStringLibrary.EndsWith` _rawexportname ".") :`false` ".") (`|GetEnumeratorNameAsString` (`self.RawFileFormat`))))))
        (:`then_1`
          (if (`self.ExportEngine`)
            (if (`BlueprintPathsLibrary.FileExists` _returnvalue)
              (`/Game/GuildLessProto/Systems/TechArt_MacroLibrary.Print_Warning` (`KismetStringLibrary.Concat_StrStr` "File already exists and should be reimported manually \n" _returnvalue))
              (else
                (`KismetRenderingLibrary.RenderTargetCreateStaticTexture2DEditorOnly` _rendertarget _rawexportname_2 (`self.RenderTargetCompression`))))))))
    (:`Is Not Valid`
      (`/Game/GuildLessProto/Systems/TechArt_MacroLibrary.Print_Error` "Export failed, render target not valid"))))

(fn `UserConstructionScript`)