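; BP_ExportBoundedActors is a placeable box volume tool that gathers the level actors inside it, presumably for export, though no export step appears here.
; The Construction Script clears SelectedActors, zeroes root relative rotation and sets up the wall cube's transform, visibility and color via custom primitive data.
; SelectActorsInBound, left unwired there, stores non-tool actors whose bounds origin lies within the Box's axis-aligned world extents.
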(fn `SelectActorsInBound`
  (bind _box (`self.Box`))
  (bind _returnvalue (`BoxComponent.GetScaledBoxExtent` _box))
  (bind _returnvalue_2 (`SceneComponent.K2_GetComponentLocation` _box))
  (`KismetArrayLibrary.Array_Clear` (`self.SelectedActors`))
  (bind _outactors (`GameplayStatics.GetAllActorsOfClass` "/Script/Engine.Actor"))
  (for _array_element _outactors
    (cast `/Game/GuildLessProto/Systems/Tools/ExportBoundedActors/BP_ExportBoundedActors` _array_element ; not select itself
      (:`CastFailed`
        (bind _x (.x (`self.GetActorBounds` _array_element false true)))
        (bind _y (.y (`self.GetActorBounds` _array_element false true)))
        (bind _z (.z (`self.GetActorBounds` _array_element false true)))
        (if (and (and (< _x (.x (+ _returnvalue_2 _returnvalue))) (> _x (.x (- _returnvalue_2 _returnvalue)))) (and (< _y (.y (+ _returnvalue_2 _returnvalue))) (> _y (.y (- _returnvalue_2 _returnvalue)))) (and (< _z (.z (+ _returnvalue_2 _returnvalue))) (> _z (.z (- _returnvalue_2 _returnvalue)))))
          (`KismetArrayLibrary.Array_Add` (`self.SelectedActors`) _array_element))))))

(fn `UserConstructionScript`
  (bind _cube (`self.Cube`))
  (bind (_r _g _b _a) (break `LinearColor` (`self.WallsColor`)))
  (`KismetArrayLibrary.Array_Clear` (`self.SelectedActors`))
  (`SceneComponent.K2_SetRelativeRotation` :`self` (`self.DefaultSceneRoot`))
  (`SceneComponent.SetRelativeScale3D` _cube (2.0 2.0 2.0))
  (`SceneComponent.K2_SetRelativeLocation` _cube (0.0 0.0 0.0) false false)
  (`PrimitiveComponent.SetCustomPrimitiveDataVector4` _cube 0 (`KismetMathLibrary.MakeVector4` _r _g _b _a))
  (`SceneComponent.SetVisibility` _cube (`self.ShowWalls`) false))