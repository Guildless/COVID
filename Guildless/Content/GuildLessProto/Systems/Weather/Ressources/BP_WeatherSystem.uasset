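; Weather system Blueprint that applies a weather preset to surface materials, directional light, post process, wind, particles and sky.
; UpdateWeather receives the preset and target components, then runs one update function per aspect.
; Surface wetness, rain and fixed or randomized wind are written to the MPC_Weather parameter collection.
; The Niagara update reads that wind back to steer rain, or destroys the component when the preset disables particles.
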(event `self.ReceiveBeginPlay`)

(fn `UpdateWeather`
  (params (WeatherPreset :type "/Game/GuildLessProto/Systems/Weather/Ressources/DA_WeatherPreset Object Reference") (AffectSurfaceMaterial :type Boolean) (LightComponent :type "LightComponent Object Reference") (PostProcess :type "PostProcessComponent Object Reference") (ParticleSystem :type "NiagaraComponent Object Reference") (SkyMesh :type "StaticMeshComponent Object Reference"))
  (`/Engine/EditorBlueprintResources/StandardMacros.IsValid` WeatherPreset
    (:`Is Valid`
      (`self.UpdateWeather_SurfaceMaterial` WeatherPreset AffectSurfaceMaterial)
      (`self.UpdateWeather_Light` LightComponent WeatherPreset)
      (`self.UpdateWeather_PostProcess` PostProcess WeatherPreset)
      (`self.UpdateWeather_Wind` WeatherPreset)
      (`self.UpdateWeather_Particles` WeatherPreset ParticleSystem)
      (`self.UpdateWeather_Sky` WeatherPreset SkyMesh))))

(fn `UpdateWeather_Light`
  (params (LightComponent :type "LightComponent Object Reference") (WeatherPreset :type "/Game/GuildLessProto/Systems/Weather/Ressources/DA_WeatherPreset Object Reference"))
  (bind (_intensity _lighttemperature _lightcolortint _dirrection) (break `/Game/GuildLessProto/Systems/Weather/Ressources/Structures/ST_Weather_Light` (`/Game/GuildLessProto/Systems/Weather/Ressources/DA_WeatherPreset.DirectionalLight` WeatherPreset)))
  (`/Engine/EditorBlueprintResources/StandardMacros.IsValid` LightComponent
    (:`Is Valid`
      (`LightComponent.SetIntensity` LightComponent _intensity)
      (`LightComponent.SetTemperature` LightComponent _lighttemperature)
      (`LightComponent.SetLightColor` LightComponent _lightcolortint true)
      (`SceneComponent.K2_SetWorldRotation` LightComponent _dirrection false false))))

(fn `UpdateWeather_Particles`
  (params (WeatherPreset :type "/Game/GuildLessProto/Systems/Weather/Ressources/DA_WeatherPreset Object Reference") (ParticleSystem :type "NiagaraComponent Object Reference"))
  (bind (_amount _durationlifetime _niagaraemitter) (break `/Game/GuildLessProto/Systems/Weather/Ressources/Structures/ST_Weather_Particles` (`/Game/GuildLessProto/Systems/Weather/Ressources/DA_WeatherPreset.Particles` WeatherPreset)))
  (if (`/Game/GuildLessProto/Systems/Weather/Ressources/DA_WeatherPreset.UseParticle` WeatherPreset)
    (`/Engine/EditorBlueprintResources/StandardMacros.IsValid` WeatherPreset
      (:`Is Valid`
        (`/Engine/EditorBlueprintResources/StandardMacros.IsValid` ParticleSystem
          (:`Is Valid`
            (`NiagaraComponent.SetAsset` ParticleSystem _niagaraemitter)
            (bind _returnvalue (`KismetMaterialLibrary.GetVectorParameterValue` "/Game/GuildLessProto/Shaders/MasterMaterial/Functions/Weather/MPC_Weather.MPC_Weather" "WindDirrectionIntensity"))
            (bind (_r _g _b _a) (break `LinearColor` _returnvalue))
            (`FXSystemComponent.SetVectorParameter` ParticleSystem "User.RainWindDirection" (* (`KismetMathLibrary.MakeVector` _r _g _b) (* _a (`KismetMathLibrary.Conv_BoolToDouble` (`/Game/GuildLessProto/Systems/Weather/Ressources/DA_WeatherPreset.UseWind` WeatherPreset)))))
            (`FXSystemComponent.SetFloatParameter` ParticleSystem "User.RainSpawnRate" _amount)))))
    (else
      (`ActorComponent.K2_DestroyComponent` ParticleSystem))))

(fn `UpdateWeather_PostProcess`
  (params (PostProcess :type "PostProcessComponent Object Reference") (WeatherPreset :type "/Game/GuildLessProto/Systems/Weather/Ressources/DA_WeatherPreset Object Reference"))
  (`/Engine/EditorBlueprintResources/StandardMacros.IsValid` PostProcess
    (:`Is Valid`
      (set `PostProcessComponent.bEnabled` (`/Game/GuildLessProto/Systems/Weather/Ressources/DA_WeatherPreset.UsePostProcess` WeatherPreset) PostProcess)
      (set `PostProcessComponent.Settings` (`/Game/GuildLessProto/Systems/Weather/Ressources/DA_WeatherPreset.Postprocess` WeatherPreset) PostProcess))))

(fn `UpdateWeather_Sky`
  (params (WeatherPreset :type "/Game/GuildLessProto/Systems/Weather/Ressources/DA_WeatherPreset Object Reference") (SkyMesh :type "StaticMeshComponent Object Reference"))
  (`/Engine/EditorBlueprintResources/StandardMacros.IsValid` WeatherPreset
    (:`Is Valid`
      (`/Engine/EditorBlueprintResources/StandardMacros.IsValid` SkyMesh
        (:`Is Valid`
          (`PrimitiveComponent.SetMaterial` SkyMesh 0 (`.SkyMaterial_2_B715856F4C97EB30497674AF95886537` (break `/Game/GuildLessProto/Systems/Weather/Ressources/Structures/ST_Weather_Sky` (`/Game/GuildLessProto/Systems/Weather/Ressources/DA_WeatherPreset.Sky` WeatherPreset)))))))))

(fn `UpdateWeather_SurfaceMaterial`
  (params (WeatherPreset :type "/Game/GuildLessProto/Systems/Weather/Ressources/DA_WeatherPreset Object Reference") (AffectSurfaceMaterial :type Boolean))
  (bind (_basecolor_desaturation _specular_wetness _roughness_wetness _rainpuddleintensity _rainpuddlessize _raindrops _raindrips _rainripples) (break `/Game/GuildLessProto/Systems/Weather/Ressources/Structures/ST_Weather_Material` (`/Game/GuildLessProto/Systems/Weather/Ressources/DA_WeatherPreset.MaterialSurface` WeatherPreset)))
  (if AffectSurfaceMaterial
    (`KismetMaterialLibrary.SetScalarParameterValue` "/Game/GuildLessProto/Shaders/MasterMaterial/Functions/Weather/MPC_Weather.MPC_Weather" "BaseColor_DeSaturation" _basecolor_desaturation)
    (`KismetMaterialLibrary.SetScalarParameterValue` "/Game/GuildLessProto/Shaders/MasterMaterial/Functions/Weather/MPC_Weather.MPC_Weather" "Specular_Wetness" _specular_wetness)
    (`KismetMaterialLibrary.SetScalarParameterValue` "/Game/GuildLessProto/Shaders/MasterMaterial/Functions/Weather/MPC_Weather.MPC_Weather" "Roughness_Wetness" _roughness_wetness)
    (`KismetMaterialLibrary.SetScalarParameterValue` "/Game/GuildLessProto/Shaders/MasterMaterial/Functions/Weather/MPC_Weather.MPC_Weather" "Rain_PuddleIntensity" _rainpuddleintensity)
    (`KismetMaterialLibrary.SetScalarParameterValue` "/Game/GuildLessProto/Shaders/MasterMaterial/Functions/Weather/MPC_Weather.MPC_Weather" "Rain_PuddleSize" _rainpuddlessize)
    (`KismetMaterialLibrary.SetScalarParameterValue` "/Game/GuildLessProto/Shaders/MasterMaterial/Functions/Weather/MPC_Weather.MPC_Weather" "Rain_Drops" _raindrops)
    (`KismetMaterialLibrary.SetScalarParameterValue` "/Game/GuildLessProto/Shaders/MasterMaterial/Functions/Weather/MPC_Weather.MPC_Weather" "Rain_Ripples" _rainripples)
    (`KismetMaterialLibrary.SetScalarParameterValue` "/Game/GuildLessProto/Shaders/MasterMaterial/Functions/Weather/MPC_Weather.MPC_Weather" "Rain_Drips" _raindrips)))

(fn `UpdateWeather_Wind`
  (params (WeatherPreset :type "/Game/GuildLessProto/Systems/Weather/Ressources/DA_WeatherPreset Object Reference"))
  (bind (_randomwinddirectionintensity _randomwindintensityrange _windintensity _winddirection) (break `/Game/GuildLessProto/Systems/Weather/Ressources/Structures/ST_Weather_Wind` (`/Game/GuildLessProto/Systems/Weather/Ressources/DA_WeatherPreset.Wind` WeatherPreset)))
  (bind (_x _y) (`KismetMathLibrary.BreakVector2D` _randomwindintensityrange))
  (`KismetMaterialLibrary.SetVectorParameterValue` "/Game/GuildLessProto/Shaders/MasterMaterial/Functions/Weather/MPC_Weather.MPC_Weather" "WindDirrectionIntensity" (select `bool` _randomwinddirectionintensity :`false` (make `LinearColor` (.x _winddirection) (.y _winddirection) (.z _winddirection) (* (`KismetMathLibrary.Conv_BoolToDouble` (`/Game/GuildLessProto/Systems/Weather/Ressources/DA_WeatherPreset.UseWind` WeatherPreset)) _windintensity)) :`true` (make `LinearColor` (`KismetMathLibrary.RandomFloatInRange` -1.0 1.0) (`KismetMathLibrary.RandomFloatInRange` -1.0 1.0) (`KismetMathLibrary.RandomFloatInRange` -0.9 0.1) (`KismetMathLibrary.RandomFloatInRange` _x _y)))))

(fn `UserConstructionScript`)