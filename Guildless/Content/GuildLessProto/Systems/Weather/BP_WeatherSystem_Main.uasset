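; Weather system actor that applies the current weather preset to its directional light, post process, Niagara particles, sky sphere and surface materials.
; A shared UpdateWeather call runs at construction, on BeginPlay and on the Update event.
; Construction also resets the root to world origin and shows a wind debug arrow when the preset uses wind.
; The arrow's rotation and length derive from MPC_Weather's wind parameter; runtime updates hide it.
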(event `self.ReceiveBeginPlay`
  (bind _currentweatherpreset (`self.CurrentWeatherPreset`))
  (`parent.ReceiveBeginPlay`)
  (`self.UpdateWeather` _currentweatherpreset true (`self.DirectionalLight`) (`self.PostProcess`) (`self.Niagara`) (`self.SkySphere`) :!label _label)
  (`self.UpdateWindDebug` _currentweatherpreset))

(event `Update`
  (goto _label))

(fn `Update_Weather`
  (`SceneComponent.K2_SetWorldTransform` (`self.DefaultSceneRoot`) (`KismetMathLibrary.MakeTransform` (0.0 0.0 0.0)) false false)
  (`self.UpdateWeather` (`self.CurrentWeatherPreset`) true (`self.DirectionalLight`) (`self.PostProcess`) (`self.Niagara`) (`self.SkySphere`))
  (`self.UpdateWindDebug` (`self.CurrentWeatherPreset`) true))

(fn `UpdateWindDebug`
  (params (WeatherPreset :type "/Game/GuildLessProto/Systems/Weather/Ressources/DA_WeatherPreset Object Reference") (Visibility :type Boolean))
  (bind _arrow (`self.Arrow`))
  (bind _usewind (`/Game/GuildLessProto/Systems/Weather/Ressources/DA_WeatherPreset.UseWind` WeatherPreset))
  (`SceneComponent.SetVisibility` _arrow (and Visibility _usewind) false)
  (`/Engine/EditorBlueprintResources/StandardMacros.IsValid` WeatherPreset
    (:`Is Valid`
      (bind _returnvalue (`KismetMaterialLibrary.GetVectorParameterValue` "/Game/GuildLessProto/Shaders/MasterMaterial/Functions/Weather/MPC_Weather.MPC_Weather" "WindDirrectionIntensity"))
      (bind (_r _g _b _a) (break `LinearColor` _returnvalue))
      (bind _returnvalue_2 (* _a (`KismetMathLibrary.Conv_BoolToDouble` _usewind) 0.001))
      (`SceneComponent.K2_SetWorldRotation` _arrow (* (* (`KismetMathLibrary.MakeRotator` _r _g _b) 360.0) _returnvalue_2) false false)
      (`SceneComponent.SetWorldScale3D` _arrow (`KismetMathLibrary.MakeVector` (+ _returnvalue_2 1.0) 1.0 1.0)))))

(fn `UserConstructionScript`
  (`parent.UserConstructionScript`)
  (`self.Update_Weather`))